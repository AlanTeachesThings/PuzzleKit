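; Input slot variant for a pipe in the interaction system that leaks liquid while off and stops when switched on.
; Off shows the Sphere and activates LiquidEffect; on hides the Sphere and deactivates the effect, both extending parent state logic.
; The Blueprint registers as the effect's CallbackHandler, receiving exported particle data to spawn randomly scaled, quickly fading splatter decals at particle positions.
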(event EventBeginPlay
  (Class|NiagaraComponent|SetVariableObject (Variables|Default|GetLiquidEffect) "CallbackHandler" self))

(event EventParticleData
  (params (Data :type Array%20of%20Basic%20Particle%20Data%20Structures) (NiagaraSystem :type Niagara%20System%20Object%20Reference) (SimulationPositionOffset :type Vector%20%28by%20ref%29 :default "0, 0, 0"))
  (for _array_element Data
    (bind _returnvalue (AddComponent|AddDecalComponent false (Math|Transform|MakeTransform (.position _array_element) (Math|Rotator|MakeRotfromX (Math|Vector|MakeVector 0.0 0.0 1.0)) (Math|Vector|MakeVector (Math|Random|RandomFloatinRange 0.1 0.25) (Math|Random|RandomFloatinRange 0.1 0.25) (Math|Random|RandomFloatinRange 0.1 0.25)))))
    (Rendering|Components|Decal|SetFadeOut _returnvalue 0.0 0.5 false)
    (Rendering|Components|Decal|SetDecalMaterial _returnvalue "/Game/InteractionSystem/Assets/VFX/Splatter_Mat.Splatter_Mat")
    (Transformation|SetWorldLocation _returnvalue (.position _array_element) false false)))

(fn ConstructionScript
  (|CallParentFunction))

(fn SetStateon
  (|CallParentFunction)
  (Rendering|SetVisibility (Variables|Default|GetSphere) false false)
  (Components|Activation|Deactivate (Variables|Default|GetLiquidEffect)))

(fn SetStateOff
  (|CallParentFunction)
  (Rendering|SetVisibility (Variables|Default|GetSphere) true false)
  (Components|Activation|Activate (Variables|Default|GetLiquidEffect) true))